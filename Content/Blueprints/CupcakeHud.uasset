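; CupcakeHud is a HUD that draws a per-player list of names and click counts on screen, apparently as a scoreboard.
; Each DrawHUD call loops over the GameState's PlayerArray and casts each entry to CupcakePlayerState to read its ClickCount.
; Name and count feed a Format Text node, and each result is drawn in black Chalkboard text, stacked vertically by array index.
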(event EventDrawHUD
  (params (SizeX :type Integer) (SizeY :type Integer))
  (for (_array_element _array_index) (Variables|/Script/Engine.GameState|GetPlayerArray (Game|GetGameState))
    (bind _ascupcakeplayerstate_c (Utilities|Casting|CastToCupcakePlayerState _array_element))
    (HUD|DrawText (Utilities|String|ToString(Text) (Utilities|Text|FormatText "" (Utilities|Text|ToText(String) (Variables|/Script/Engine.PlayerState|GetPlayerName _array_element)) (Utilities|Text|ToText(Integer) (Variables|/Game/Blueprints/CupcakePlayerState.CupcakePlayerState_C|GetClickCount _ascupcakeplayerstate_c) "HalfToEven"))) "(R=0.000000,G=0.000000,B=0.000000,A=1.000000)" 0.0 (Math|Conversions|ToFloat(Integer) (* _array_index 30)) "/Game/Fonts/Chalkboard.Chalkboard" 1.5 false)))

(fn ConstructionScript)