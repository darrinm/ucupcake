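; Player state that tracks one player's cupcake click count and feeds each click into the shared cupcake total.
; CupcakeClicked calls OnCupcakeClicked, which increments ClickCount and adds one to the count on CupcakeGameState.
; On remote clients it also increments ClickCount immediately as a prediction until the server's authoritative value arrives.
; The ClickCount RepNotify is empty.
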(event Custom|OnCupcakeClicked
  (Variables|PlayerState|SetClickCount (+ (Variables|PlayerState|GetClickCount) 1))
  (bind _ascupcakegamestate_c (Utilities|Casting|CastToCupcakeGameState (Game|GetGameState)))
  (Default|AddtoCupcakeCount _ascupcakegamestate_c 1.0))

(fn ConstructionScript)

(fn OnRepClickCount)

(fn CupcakeClicked
  (CallFunction|OnCupcakeClicked)
  ;[1 1 1] Increment client value immediately while waiting for authoritative value from server.
  (Networking|SwitchHasAuthority
    (:Remote
      (Variables|PlayerState|SetClickCount (+ (Variables|PlayerState|GetClickCount) 1)))))