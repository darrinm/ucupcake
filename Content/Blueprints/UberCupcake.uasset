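; UberCupcake is a clickable actor that shows a hand cursor on hover and changes scale while the left mouse button is held.
; Cursor-over events on Shape_Cube switch the player cursor.
; The LeftMouseButton input action traces under the cursor and applies PressedScale on any hit, without checking which actor, then restores NormalScale on release.
; The component's click and release events are empty, with a note that OnClicked misses double-clicks.
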(event OnClicked(Shape_Cube)
  (params (TouchedComponent :type Primitive%20Component%20Object%20Reference))
  ;[1 1 1] Doesn't catch double-click!
)

(event OnBeginCursorOver(Shape_Cube)
  (params (TouchedComponent :type Primitive%20Component%20Object%20Reference))
  (Variables|/Script/Engine.PlayerController|SetCurrentMouseCursor (Game|GetPlayerController 0) "Hand"))

(event OnEndCursorOver(Shape_Cube)
  (params (TouchedComponent :type Primitive%20Component%20Object%20Reference))
  (Variables|/Script/Engine.PlayerController|SetCurrentMouseCursor (Game|GetPlayerController 0) "Default"))

(event OnReleased(Shape_Cube)
  (params (TouchedComponent :type Primitive%20Component%20Object%20Reference))
  ;[1 1 1] Doesn't catch double-click!
)

(event Input|ActionEvents|InputActionLeftMouseButton
  (bind _pressedscale (Variables|Default|GetPressedScale))
  (bind _normalscale (Variables|Default|GetNormalScale))
  (:Pressed
    (if (.ReturnValue (Game|Player|GetHitResultUnderCursorbyChannel (Game|GetPlayerController 0) "TraceTypeQuery1" true))
      (Transformation|SetActorScale3D (Math|Vector|MakeVector _pressedscale _pressedscale _pressedscale))))
  (:Released
    (Transformation|SetActorScale3D (Math|Vector|MakeVector _normalscale _normalscale _normalscale))))

(fn ConstructionScript)